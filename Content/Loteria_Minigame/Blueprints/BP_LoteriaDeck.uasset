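; BP_LoteriaDeck is the deck actor for a Lotería minigame, building a randomized board of cards when play begins.
; It spawns sixteen BP_LoteriaCard actors at its own transform, initializes each by index and collects them in Deck.
; A working copy, PlayerDeck, is drawn from at random without repeats to fill BoardMap by slot number.
; LayCards then offsets each card into grid columns and rows using the slot's modulo and division by four.
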(event `self.ReceiveBeginPlay`
  (for _index (range 1 17)
    (bind _returnvalue (`|SpawnActorFromClass` "/Game/Loteria_Minigame/Blueprints/BP_LoteriaCard.BP_LoteriaCard_C" (`self.GetTransform`) "Undefined" "MultiplyWithRoot" null null))
    (`/Game/Loteria_Minigame/Blueprints/BP_LoteriaCard.InitializeCard` _returnvalue _index)
    (`KismetArrayLibrary.Array_AddUnique` (`self.Deck`)))
  (set `self.PlayerDeck` (`self.Deck`))
  (for _index_2 (range 1 17)
    (`BlueprintMapLibrary.Map_Add` (`self.BoardMap`) _index_2 (`KismetArrayLibrary.Array_Random` (`self.PlayerDeck`)))
    (`KismetArrayLibrary.Array_RemoveItem` (`self.PlayerDeck`)))
  (`self.LayCards`))

(fn `LayCards`
  (bind _keys (`BlueprintMapLibrary.Map_Keys` (`self.BoardMap`)))
  (for _array_element _keys
    (bind _value (`BlueprintMapLibrary.Map_Find` (`self.BoardMap`) _array_element))
    (`self.K2_SetActorLocation` _value (+ (`self.K2_GetActorLocation` _value) (`KismetMathLibrary.MakeVector` (select `int` (mod _array_element 4) :`0` 0.0 :`1` 100.0 :`2` 200.0 :`3` 300.0) (select `int` (/ _array_element 4) :`0` 0.0 :`1` 125.0 :`2` 250.0 :`3` 375.0))) false false)))

(fn `UserConstructionScript`)