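; Lotería minigame board actor that builds a randomized 4x4 grid of cards and detects winning patterns.
; On BeginPlay it spawns 16 BP_LoteriaCard actors, draws them randomly into a position-keyed map, lays them out and triggers their previews.
; CheckWin marks a card flipped, then uses index arithmetic to test its row, column and neighboring 2x2 squares.
; A completed pattern calls GameWon on the level's BP_LoteriaDeck.
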(event `self.ReceiveBeginPlay`
  (bind _currrandcard (`self.CurrRandCard`))
  (bind _playerdeck (`self.PlayerDeck`))
  ; Create Deck of Cards
  (`KismetSystemLibrary.Delay` 3.0)
  (bind _returnvalue (`GameplayStatics.GetActorOfClass` "/Game/Blueprints/Loteria_Minigame/Blueprints/BP_LoteriaDeck.BP_LoteriaDeck_C"))
  (set `self.DeckRef` _returnvalue)
  (for _index (range 1 17)
    (bind _returnvalue_2 (`|SpawnActorFromClass` "/Game/Blueprints/Loteria_Minigame/Blueprints/BP_LoteriaCard.BP_LoteriaCard_C" (`self.GetTransform`) "AlwaysSpawn" "MultiplyWithRoot" null null))
    (`/Game/Blueprints/Loteria_Minigame/Blueprints/BP_LoteriaCard.InitializeCard` _returnvalue_2 self _index)
    (`KismetArrayLibrary.Array_AddUnique` (`self.Deck`) _returnvalue_2))
  ; Create Board
  (set `self.PlayerDeck` (`self.Deck`))
  (if (`KismetArrayLibrary.Array_IsNotEmpty` _playerdeck) :!label _label
    (set `self.CurrRandCard` (`KismetArrayLibrary.Array_Random` _playerdeck))
    (`BlueprintMapLibrary.Map_Add` (`self.BoardMap`) (`self.Count`) _currrandcard)
    (`KismetArrayLibrary.Array_RemoveItem` (`self.PlayerDeck`) _currrandcard)
    (`KismetSystemLibrary.Delay` 0.0)
    (`/Engine/EditorBlueprintResources/StandardMacros.IncrementInt` (`self.Count`)
      (:`  `
        (goto _label)))
    (else
      (`self.LayCards`)
      (`KismetSystemLibrary.Delay` 1.0)
      (bind _keys (`BlueprintMapLibrary.Map_Keys` (`self.BoardMap`)))
      (bind _output_get (set `self.Keys` _keys))
      (for _array_element _output_get
        (`/Game/Blueprints/Loteria_Minigame/Blueprints/BP_LoteriaCard.Preview` (`BlueprintMapLibrary.Map_Find` (`self.BoardMap`) _array_element))
        (`KismetSystemLibrary.Delay` 3.0)))))

(event `CheckWin`
  (params (CardLoc :type Integer))
  (bind _latestcardloc (`self.LatestCardLoc`))
  (bind _latestcardloc_2 (`self.LatestCardLoc`))
  (bind _latestcardloc_3 (`self.LatestCardLoc`))
  ; Check Win Cons
  (bind _output_get (set `self.LatestCardLoc` CardLoc))
  (set `/Game/Blueprints/Loteria_Minigame/Blueprints/BP_LoteriaCard.CardFlipped` true (`BlueprintMapLibrary.Map_Find` (`self.BoardMap`) _output_get))
  (`self.RowCheck` _latestcardloc_3)
  (`self.ColumnCheck` _latestcardloc_3)
  (if (!= (mod _latestcardloc_3 4) 3)
    (`self.BRCorner` _latestcardloc)
    (`self.BLCorner` _latestcardloc))
  (if (!= (mod (`self.LatestCardLoc`) 4) 0)
    (`self.TLCorner` _latestcardloc_2)
    (`self.TRCorner` _latestcardloc_2)))

(fn `BLCorner`
  (params (CardLoc :type Integer))
  (if (< CardLoc 11)
    (`KismetSystemLibrary.PrintString` "BL")
    (if (and (`/Game/Blueprints/Loteria_Minigame/Blueprints/BP_LoteriaCard.CardFlipped` (`BlueprintMapLibrary.Map_Find` (`self.BoardMap`) (+ (`local.CardLoc`) 1))) (`/Game/Blueprints/Loteria_Minigame/Blueprints/BP_LoteriaCard.CardFlipped` (`BlueprintMapLibrary.Map_Find` (`self.BoardMap`) (+ (`local.CardLoc`) 4))) (`/Game/Blueprints/Loteria_Minigame/Blueprints/BP_LoteriaCard.CardFlipped` (`BlueprintMapLibrary.Map_Find` (`self.BoardMap`) (+ (`local.CardLoc`) 5))))
      (`KismetSystemLibrary.PrintString` "BL")
      (`/Game/Blueprints/Loteria_Minigame/Blueprints/BP_LoteriaDeck.GameWon` (`self.DeckRef`) false))))

(fn `BRCorner`
  (params (CardLoc :type Integer))
  (if (> CardLoc 4)
    (`KismetSystemLibrary.PrintString` "BR")
    (if (and (`/Game/Blueprints/Loteria_Minigame/Blueprints/BP_LoteriaCard.CardFlipped` (`BlueprintMapLibrary.Map_Find` (`self.BoardMap`) (+ (`local.CardLoc`) 1))) (`/Game/Blueprints/Loteria_Minigame/Blueprints/BP_LoteriaCard.CardFlipped` (`BlueprintMapLibrary.Map_Find` (`self.BoardMap`) (+ (`local.CardLoc`) -3))) (`/Game/Blueprints/Loteria_Minigame/Blueprints/BP_LoteriaCard.CardFlipped` (`BlueprintMapLibrary.Map_Find` (`self.BoardMap`) (+ (`local.CardLoc`) -4))))
      (`KismetSystemLibrary.PrintString` "BR")
      (`/Game/Blueprints/Loteria_Minigame/Blueprints/BP_LoteriaDeck.GameWon` (`self.DeckRef`) false))))

(fn `ColumnCheck`
  (params (CardLoc :type Integer))
  (locals (Flag :type Boolean :default true) (CheckCon :type Integer))
  (set `local.CheckCon` (mod CardLoc 4))
  (for _array_element (`self.Keys`)
    (if (== (mod _array_element 4) (`local.CheckCon`))
      (if (not (`/Game/Blueprints/Loteria_Minigame/Blueprints/BP_LoteriaCard.CardFlipped` (`BlueprintMapLibrary.Map_Find` (`self.BoardMap`) _array_element)))
        (set `local.Flag` false))))
  (if (`local.Flag`)
    (`KismetSystemLibrary.PrintString` "Column")
    (`/Game/Blueprints/Loteria_Minigame/Blueprints/BP_LoteriaDeck.GameWon` (`self.DeckRef`) (`self.P1?`))))

(fn `LayCards`
  (locals (CurrIndex :type Integer))
  (bind _keys (`BlueprintMapLibrary.Map_Keys` (`self.BoardMap`)))
  (for (_array_element _array_index) _keys
    (bind _output_get (set `local.CurrIndex` _array_index))
    (bind _value (`BlueprintMapLibrary.Map_Find` (`self.BoardMap`) _output_get))
    (set `/Game/Blueprints/Loteria_Minigame/Blueprints/BP_LoteriaCard.CardLoc` _array_element _value)
    (`self.K2_SetActorLocation` _value (+ (`self.K2_GetActorLocation` _value) (`KismetMathLibrary.MakeVector` (select `int` (mod _output_get 4) :`0` 0.0 :`1` 375.0 :`2` 750.0 :`3` 1125.0) (select `int` (/ _output_get 4) :`0` 0.0 :`1` 375.0 :`2` 750.0 :`3` 1125.0))) false false)))

(fn `RowCheck`
  (params (CardLoc :type Integer))
  (locals (CheckCon :type Integer) (Flag :type Boolean :default true))
  (set `local.CheckCon` (/ CardLoc 4))
  (for _array_element (`self.Keys`)
    (if (== (/ _array_element 4) (`local.CheckCon`))
      (if (not (`/Game/Blueprints/Loteria_Minigame/Blueprints/BP_LoteriaCard.CardFlipped` (`BlueprintMapLibrary.Map_Find` (`self.BoardMap`) _array_element)))
        (set `local.Flag` false))))
  (if (`local.Flag`)
    (`KismetSystemLibrary.PrintString` "Row")
    (`/Game/Blueprints/Loteria_Minigame/Blueprints/BP_LoteriaDeck.GameWon` (`self.DeckRef`) false)))

(fn `TLCorner`
  (params (CardLoc :type Integer))
  (if (< CardLoc 11)
    (`KismetSystemLibrary.PrintString` "TL")
    (if (and (`/Game/Blueprints/Loteria_Minigame/Blueprints/BP_LoteriaCard.CardFlipped` (`BlueprintMapLibrary.Map_Find` (`self.BoardMap`) (+ (`local.CardLoc`) -1))) (`/Game/Blueprints/Loteria_Minigame/Blueprints/BP_LoteriaCard.CardFlipped` (`BlueprintMapLibrary.Map_Find` (`self.BoardMap`) (+ (`local.CardLoc`) 3))) (`/Game/Blueprints/Loteria_Minigame/Blueprints/BP_LoteriaCard.CardFlipped` (`BlueprintMapLibrary.Map_Find` (`self.BoardMap`) (+ (`local.CardLoc`) 4))))
      (`KismetSystemLibrary.PrintString` "TL")
      (`/Game/Blueprints/Loteria_Minigame/Blueprints/BP_LoteriaDeck.GameWon` (`self.DeckRef`) false))))

(fn `TRCorner`
  (params (CardLoc :type Integer))
  (if (> CardLoc 4)
    (`KismetSystemLibrary.PrintString` "TR")
    (if (and (`/Game/Blueprints/Loteria_Minigame/Blueprints/BP_LoteriaCard.CardFlipped` (`BlueprintMapLibrary.Map_Find` (`self.BoardMap`) (+ (`local.CardLoc`) -4))) (`/Game/Blueprints/Loteria_Minigame/Blueprints/BP_LoteriaCard.CardFlipped` (`BlueprintMapLibrary.Map_Find` (`self.BoardMap`) (+ (`local.CardLoc`) -5))) (`/Game/Blueprints/Loteria_Minigame/Blueprints/BP_LoteriaCard.CardFlipped` (`BlueprintMapLibrary.Map_Find` (`self.BoardMap`) (+ (`local.CardLoc`) -1))))
      (`KismetSystemLibrary.PrintString` "TR")
      (`/Game/Blueprints/Loteria_Minigame/Blueprints/BP_LoteriaDeck.GameWon` (`self.DeckRef`) false))))

(fn `UserConstructionScript`)