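; A board card in the Lotería minigame that flips face up when it receives a GroundPound event.
; InitializeCard loads its data from DT_Cards by ID and applies the face texture through a dynamic material instance.
; FlipCard keeps the card flipped and asks the board to check for a win if the deck's DisplayedLocs contains its ID.
; Otherwise it rotates back after a short delay, as does Preview, which briefly reveals the card.
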(event `self.ReceiveBeginPlay`
  (bind _returnvalue (`KismetMaterialLibrary.CreateDynamicMaterialInstance` "/Game/Materials/MI_CardFace.MI_CardFace"))
  (bind _output_get (set `self.CardFaceMI` _returnvalue))
  (`PrimitiveComponent.SetMaterial` (`self.CardFace`) 0 _output_get)
  (bind _returnvalue_2 (`GameplayStatics.GetActorOfClass` "/Game/Blueprints/Loteria_Minigame/Blueprints/BP_LoteriaDeck.BP_LoteriaDeck_C"))
  (set `self.DeckRef` _returnvalue_2))

(event `Preview`
  (`self.K2_SetActorRotation` (struct :`Pitch` 180.0))
  (`KismetSystemLibrary.Delay` 2.0)
  (`self.K2_SetActorRotation` (struct)))

(event `FlipCard`
  (if (`KismetArrayLibrary.Array_Contains` (`/Game/Blueprints/Loteria_Minigame/Blueprints/BP_LoteriaDeck.DisplayedLocs` (`self.DeckRef`)) (`.CardID_9_C812FB3143E5609DF347A985035602B0` (break `/Game/Blueprints/Loteria_Minigame/Structs/S_CardData` (`self.CardData`))))
    (`self.K2_SetActorRotation` (struct :`Pitch` 180.0))
    (set `self.CardFlipped` true)
    (`KismetSystemLibrary.Delay` 0.0)
    (`/Game/Blueprints/Loteria_Minigame/Blueprints/BP_LoteriaBoard.CheckWin` (`self.Board Ref`) (`self.CardLoc`))
    (else
      (`self.K2_SetActorRotation` (struct :`Pitch` 180.0))
      (`KismetSystemLibrary.Delay` 2.0)
      (`self.K2_SetActorRotation` (struct)))))

(event `/Game/Blueprints/Player/BPI_Interactions.GroundPound`
  (`self.FlipCard`))

(fn `InitializeCard`
  (params (BoardRef :type "/Game/Blueprints/Loteria_Minigame/Blueprints/BP_LoteriaBoard Object Reference") (NewCardID :type Integer))
  (set `self.CardFlipped` false)
  (set `self.Board Ref` BoardRef)
  (bind _returnvalue (`|GetDataTableRow` "/Game/Blueprints/Loteria_Minigame/DataTables/DT_Cards.DT_Cards" (`KismetStringLibrary.Conv_StringToName` (`KismetStringLibrary.Conv_IntToString` NewCardID)))
    (:`then`
      (bind _output_get (set `self.CardData` _returnvalue))
      (`MaterialInstanceDynamic.SetTextureParameterValue` (`self.CardFaceMI`) "Face" (`.CardTexture_8_D2832A5B447311D8FACDF08856AEBB28` (break `/Game/Blueprints/Loteria_Minigame/Structs/S_CardData` _output_get))))))

(fn `UserConstructionScript`)