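; Card deck actor for the Lotería minigame that deals and cycles face-up cards until the game is won.
; BeginPlay spawns 16 stacked cards with sequential IDs, then starts the self-repeating ShowNewCard loop after a delay.
; Each tick of that loop moves the top card into one of five spaced slots, later recycling replaced cards to the deck's end in round-robin order.
; Displayed card IDs are tracked alongside the actors, and GameWon stops the loop.
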(event `self.ReceiveBeginPlay`
  (for _index (range 1 17)
    (bind _returnvalue (`|SpawnActorFromClass` "/Game/Blueprints/Loteria_Minigame/Blueprints/BP_LoteriaCard.BP_LoteriaCard_C" (`KismetMathLibrary.MakeTransform` (`KismetMathLibrary.MakeVector` (.x (.location (`self.GetTransform`))) (.y (.location (`self.GetTransform`))) (+ (* _index 2.0) (.z (.location (`self.GetTransform`))))) (.rotation (`self.GetTransform`)) (.scale (`self.GetTransform`))) "AlwaysSpawn" "MultiplyWithRoot" null null))
    (`/Game/Blueprints/Loteria_Minigame/Blueprints/BP_LoteriaCard.InitializeCard` _returnvalue null _index)
    (`KismetArrayLibrary.Array_AddUnique` (`self.Deck`) _returnvalue)
    (`KismetSystemLibrary.Delay` 5.0)
    (`self.ShowNewCard`)))

(event `ShowNewCard`
  (bind (_returnvalue_x _returnvalue_y _returnvalue_z) (`KismetMathLibrary.BreakVector` (`self.K2_GetActorLocation`)))
  (bind (_returnvalue_x_2 _returnvalue_y_2 _returnvalue_z_2) (`KismetMathLibrary.BreakVector` (`self.K2_GetActorLocation`)))
  (bind _returnvalue (mod (`self.FlipCount`) 5))
  (bind _output (`|GetArrayItem` (`self.Deck`)))
  (bind _output_2 (`|GetArrayItem` (`self.Deck`)))
  (if (`self.Show New Card?`)
    (if (<= (`self.Count`) 5)
      (`KismetArrayLibrary.Array_Add` (`self.DisaplayedCards`) _output)
      (`KismetArrayLibrary.Array_Add` (`self.DisplayedLocs`) (`.CardID_9_C812FB3143E5609DF347A985035602B0` (break `/Game/Blueprints/Loteria_Minigame/Structs/S_CardData` (`/Game/Blueprints/Loteria_Minigame/Blueprints/BP_LoteriaCard.CardData` _output))))
      (`KismetArrayLibrary.Array_RemoveItem` (`self.Deck`) _output)
      (`self.K2_SetActorRotation` (`|GetArrayItem` (`self.DisaplayedCards`) (mod (`self.Count`) 5)) (struct :`Pitch` 180.0 :`Yaw` 90.0) false)
      (`self.K2_SetActorLocation` (`|GetArrayItem` (`self.DisaplayedCards`) (mod (`self.Count`) 5)) (`KismetMathLibrary.MakeVector` _returnvalue_x_2 (`self.CardLocFinder` _returnvalue_y_2 (`self.Count`)) _returnvalue_z_2) false false)
      (`/Engine/EditorBlueprintResources/StandardMacros.IncrementInt` (`self.Count`)
        (:`  `
          _))
      (else
        (`self.K2_SetActorLocationAndRotation` (`|GetArrayItem` (`self.DisaplayedCards`) (mod (`self.FlipCount`) 5)) (`self.K2_GetActorLocation`) (struct :`Yaw` 90.0) false false)
        (`KismetArrayLibrary.Array_Add` (`self.Deck`) (`|GetArrayItem` (`self.DisaplayedCards`) (mod (`self.FlipCount`) 5)))
        (`KismetArrayLibrary.Array_Set` (`self.DisaplayedCards`) _returnvalue _output_2)
        (`KismetArrayLibrary.Array_Set` (`self.DisplayedLocs`) _returnvalue (`.CardID_9_C812FB3143E5609DF347A985035602B0` (break `/Game/Blueprints/Loteria_Minigame/Structs/S_CardData` (`/Game/Blueprints/Loteria_Minigame/Blueprints/BP_LoteriaCard.CardData` _output_2))))
        (`self.K2_SetActorRotation` _output_2 (struct :`Pitch` 180.0 :`Yaw` 90.0) false)
        (`KismetArrayLibrary.Array_RemoveItem` (`self.Deck`) _output_2)
        (`self.K2_SetActorLocation` (`|GetArrayItem` (`self.DisaplayedCards`) (mod (`self.FlipCount`) 5)) (`KismetMathLibrary.MakeVector` _returnvalue_x (`self.CardLocFinder` _returnvalue_y (`self.FlipCount`)) _returnvalue_z) false false)
        (`/Engine/EditorBlueprintResources/StandardMacros.IncrementInt` (`self.FlipCount`)
          (:`  `
            _))))
    (`KismetSystemLibrary.Delay` 1.0)
    (`self.ShowNewCard`)))

(fn `CardLocFinder`
  (params (A :type "Float (double-precision)") (A1 :type Integer))
  (returns (ReturnValue :type "Float (double-precision)"))
  (return (+ A (`KismetMathLibrary.Conv_IntToDouble` (* (+ (mod A1 5) 1) 375)))))

(fn `GameWon`
  (set `self.Show New Card?` false))

(fn `UserConstructionScript`)