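; BP_Arms is a player arms Blueprint that receives four-direction input for what the IMC_BopIt mapping context suggests is a Bop It-style game.
; On BeginPlay it adds that Enhanced Input mapping context to the local player subsystem of its player controller.
; The top, right, bottom and left input actions currently only print debug key letters, with no gameplay logic attached.
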(event `self.ReceiveBeginPlay`
  (bind _asplayer_controller (cast `PlayerController` (`self.GetController`)))
  (bind _returnvalue (pcsubsystem `EnhancedInputLocalPlayerSubsystem` _asplayer_controller))
  (`/Engine/EditorBlueprintResources/StandardMacros.IsValid` _returnvalue
    (:`Is Valid`
      (`EnhancedInputSubsystemInterface.AddMappingContext` _returnvalue "/Game/Blueprints/Player/Controls/IMC_BopIt.IMC_BopIt" 0 (struct)))))

(event `EnhancedInput|/Game/Blueprints/Player/Controls/Inputs/IA_Top`
  (params (ActionValue :type Boolean) (ElapsedSeconds :type "Float (double-precision)") (TriggeredSeconds :type "Float (double-precision)") (InputAction :type "InputAction Object Reference" :default "/Game/Blueprints/Player/Controls/Inputs/IA_Top.IA_Top"))
  (:`Triggered`
    (`KismetSystemLibrary.PrintString` "W")))

(event `EnhancedInput|/Game/Blueprints/Player/Controls/Inputs/IA_Right`
  (params (ActionValue :type Boolean) (ElapsedSeconds :type "Float (double-precision)") (TriggeredSeconds :type "Float (double-precision)") (InputAction :type "InputAction Object Reference" :default "/Game/Blueprints/Player/Controls/Inputs/IA_Right.IA_Right"))
  (:`Triggered`
    (`KismetSystemLibrary.PrintString` "D")))

(event `EnhancedInput|/Game/Blueprints/Player/Controls/Inputs/IA_Bottom`
  (params (ActionValue :type Boolean) (ElapsedSeconds :type "Float (double-precision)") (TriggeredSeconds :type "Float (double-precision)") (InputAction :type "InputAction Object Reference" :default "/Game/Blueprints/Player/Controls/Inputs/IA_Bottom.IA_Bottom"))
  (:`Triggered`
    (`KismetSystemLibrary.PrintString` "S")))

(event `EnhancedInput|/Game/Blueprints/Player/Controls/Inputs/IA_Left`
  (params (ActionValue :type Boolean) (ElapsedSeconds :type "Float (double-precision)") (TriggeredSeconds :type "Float (double-precision)") (InputAction :type "InputAction Object Reference" :default "/Game/Blueprints/Player/Controls/Inputs/IA_Left.IA_Left"))
  (:`Triggered`
    (`KismetSystemLibrary.PrintString` "A")))

(fn `UserConstructionScript`)