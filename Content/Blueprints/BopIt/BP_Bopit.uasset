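; BP_Bopit runs a Bop It-style reaction game, picking random actions that are only printed as numbers.
; A matching CompareInput call adds score, shortens and restarts the lose timer, then picks another action; wrong input is ignored.
; Timer expiry calls GameEnd, which shows the W_BopItScore widget in UI-only input mode.
; At the minimum-time threshold, the match branch only clamps Time, without restarting the timer or picking an action.
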(event `CompareInput`
  (params (PlayerInput :type Integer))
  (bind _returnvalue (- (`self.Time`) 0.1))
  (if (== PlayerInput (`self.ActionDue`))
    (`/Engine/EditorBlueprintResources/StandardMacros.IncrementInt` (`self.Score`)
      (:`  `
        (`KismetSystemLibrary.K2_ClearAndInvalidateTimerHandle` (`self.LoseHandler`))
        (if (> _returnvalue 1.0)
          (set `self.Time` _returnvalue)
          (bind _returnvalue_2 (`KismetSystemLibrary.K2_SetTimerDelegate` (delegate `GameEnd`) (`self.Time`)))
          (set `self.LoseHandler` _returnvalue_2)
          (`self.NewAction`)
          (else
            (set `self.Time` 0.5)))))))

(event `StartGame`
  (bind _returnvalue (`KismetSystemLibrary.K2_SetTimerDelegate` (delegate `GameEnd`) (`self.Time`)))
  (set `self.LoseHandler` _returnvalue)
  (`self.NewAction`))

(event `GameEnd`
  (bind _returnvalue (`|CreateWidget` "/Game/Widgets/W_BopItScore.W_BopItScore_C"))
  (`UserWidget.AddToViewport` _returnvalue 0)
  (`WidgetBlueprintLibrary.SetInputMode_UIOnlyEx` (`GameplayStatics.GetPlayerController` 0) _returnvalue))

(fn `NewAction`
  (bind _output_get (set `self.ActionDue` (`KismetMathLibrary.RandomIntegerInRange` 0 4)))
  (switch `int` _output_get
    (:`Default`
      (`KismetSystemLibrary.PrintString` "Out of Range"))
    (:`0`
      (`KismetSystemLibrary.PrintString` "0"))
    (:`1`
      (`KismetSystemLibrary.PrintString` "1"))
    (:`2`
      (`KismetSystemLibrary.PrintString` "2"))
    (:`3`
      (`KismetSystemLibrary.PrintString` "3"))
    (:`4`
      (`KismetSystemLibrary.PrintString` "4"))))

(fn `UserConstructionScript`)